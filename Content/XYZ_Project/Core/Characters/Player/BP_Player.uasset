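; Player character Blueprint whose only visible logic is two debug helpers for comparing capsule and mesh facing.
; PrintForwardVectors prints both forward vectors on screen, blue for the capsule and red for the mesh.
; DrawForwardVectors draws matching arrows, the mesh's longer, both starting at the capsule's relative location, which both of its printouts also report.
; Tick and the construction script are empty, and neither helper is called here.
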(event `self.ReceiveTick`
  (params (DeltaSeconds :type "Float (single-precision)")))

(fn `DrawForwardVectors`
  (bind _relativelocation (`SceneComponent.RelativeLocation` (`self.CapsuleComponent`)))
  (bind _relativelocation_2 (`SceneComponent.RelativeLocation` (`self.CapsuleComponent`)))
  (`KismetSystemLibrary.PrintString` (`KismetStringLibrary.Concat_StrStr` "Capsule Forward Vector Location:" (`KismetStringLibrary.Conv_VectorToString` _relativelocation)) true true (struct :`B` 1.0 :`A` 1.0) 0.0)
  (`KismetSystemLibrary.DrawDebugArrow` _relativelocation (+ (* (`SceneComponent.GetForwardVector` (`self.CapsuleComponent`)) 50.0) (`SceneComponent.RelativeLocation` (`self.CapsuleComponent`))) 10.0 (struct :`B` 1.0 :`A` 1.0))
  (`KismetSystemLibrary.PrintString` (`KismetStringLibrary.Concat_StrStr` "Mesh Forward Vector Location:" (`KismetStringLibrary.Conv_VectorToString` _relativelocation_2)) true true (struct :`R` 1.0 :`A` 1.0) 0.0)
  (`KismetSystemLibrary.DrawDebugArrow` _relativelocation_2 (+ (* (`SceneComponent.GetForwardVector` (`self.Mesh`)) 100.0) (`SceneComponent.RelativeLocation` (`self.CapsuleComponent`))) 10.0 (struct :`R` 1.0 :`A` 1.0)))

(fn `PrintForwardVectors`
  (`KismetSystemLibrary.PrintString` (`KismetStringLibrary.Concat_StrStr` "Capsule Forward Vector:" (`KismetStringLibrary.Conv_VectorToString` (`SceneComponent.GetForwardVector` (`self.CapsuleComponent`)))) true true (struct :`B` 1.0 :`A` 1.0) 0.0)
  (`KismetSystemLibrary.PrintString` (`KismetStringLibrary.Concat_StrStr` "Mesh Forward Vector:" (`KismetStringLibrary.Conv_VectorToString` (`SceneComponent.GetForwardVector` (`self.Mesh`)))) true true (struct :`R` 1.0 :`A` 1.0) 0.0))

(fn `UserConstructionScript`)